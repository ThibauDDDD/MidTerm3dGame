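; Zombie enemy that hunts the player and dies when shot.
; From BeginPlay it uses AI MoveTo toward the player character; each successful reach takes one Life, calls the player's Init and restarts the chase after a short delay.
; A failed move has no retry.
; A hit from BP_Bullet plays a death animation and impact sound, stops movement, then destroys the zombie after a delay.
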(event Custom|ChasePlayer
  (bind _bp_thirdpersoncharacter (Variables|Default|GetBP_ThirdPersonCharacter))
  (AI|AIMoveTo self "0, 0, 0" (Game|GetPlayerCharacter 0) 5.0 false
    (:OnSuccess
      (Variables|/Game/ThirdPerson/Blueprints/BP_ThirdPersonCharacter.BP_ThirdPersonCharacter_C|SetLife _bp_thirdpersoncharacter (- (Variables|/Game/ThirdPerson/Blueprints/BP_ThirdPersonCharacter.BP_ThirdPersonCharacter_C|GetLife _bp_thirdpersoncharacter) 1))
      (Default|Init _bp_thirdpersoncharacter)
      (Utilities|FlowControl|Delay 1.0)
      (CallFunction|ChasePlayer))))

(event EventBeginPlay
  (bind _asbp_third_person_character (Utilities|Casting|CastToBP_ThirdPersonCharacter (Game|GetPlayerCharacter 0)))
  (Variables|Default|SetBP_ThirdPersonCharacter _asbp_third_person_character)
  (CallFunction|ChasePlayer))

(event Collision|EventActorBeginOverlap
  (params (OtherActor :type Actor%20Object%20Reference)))

(event EventTick
  (params (DeltaSeconds :type Float%20%28single-precision%29)))

(event Collision|EventHit
  (params (MyComp :type Primitive%20Component%20Object%20Reference) (Other :type Actor%20Object%20Reference) (OtherComp :type Primitive%20Component%20Object%20Reference) (bSelfMoved :type Boolean) (HitLocation :type Vector :default "0, 0, 0") (HitNormal :type Vector :default "0, 0, 0") (NormalImpulse :type Vector :default "0, 0, 0") (Hit :type Hit%20Result%20Structure%20%28by%20ref%29))
  (if (== (Utilities|GetClass Other) "/Game/BP_Bullet.BP_Bullet_C")
    (Components|Animation|PlayAnimation (Variables|Character|GetMesh) "/Game/Anim3rdPersonView/Death_2.Death_2" false)
    (Components|Movement|StopMovementImmediately (Variables|Character|GetCharacterMovement))
    (Audio|PlaySound2D "/Game/MilitaryWeapSilver/Sound/Knife/Cues/Knife_ImpactBody_Cue.Knife_ImpactBody_Cue" 1.0 1.0 0.0 0 0)
    (Utilities|FlowControl|Delay 1.0)
    (Actor|DestroyActor)))

(fn ConstructionScript)